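; Animated clock actor that rotates its second, minute and hour hands and starts a ticking sound on BeginPlay.
; A ClockTick timeline sets the second hand's relative pitch and loops by calling StartAgain when it finishes.
; Tick also keeps calling Play on that timeline and adds fixed pitch steps to the minute and hour hands each frame, so their speed depends on frame rate rather than real time.
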(event Custom|Start%20again
  (bind _clock_tick (Timeline|Clock%20Tick PlayFromStart)
    (:Update
      (Transformation|SetRelativeRotation (Variables|Default|GetSM_Clock_Ticker_Seconds) (Math|Rotator|MakeRotator 0.0 _clock_tick 0.0) false false))
    (:Finished
      (CallFunction|StartAgain))))

(event EventBeginPlay
  (Audio|Components|Audio|Play (Variables|Default|GetAC_Clock_Tick) 0.0))

(event EventTick
  (params (DeltaSeconds :type Float%20%28single-precision%29))
  (Utilities|FlowControl|Sequence
    (:then_0
      (bind _clock_tick (Timeline|Clock%20Tick Play)
        (:Update
          (Transformation|SetRelativeRotation (Variables|Default|GetSM_Clock_Ticker_Seconds) (Math|Rotator|MakeRotator 0.0 _clock_tick 0.0) false false))
        (:Finished
          (CallFunction|StartAgain))))
    (:then_1
      (Transformation|AddLocalRotation (Variables|Default|GetSM_Clock_Ticker_Hour) (Math|Rotator|MakeRotator 0.0 -0.1 0.0) false false)
      (Transformation|AddLocalRotation (Variables|Default|GetSM_Clock_Ticker_Minute) (Math|Rotator|MakeRotator 0.0 -0.6 0.0) false false))))

(fn ConstructionScript)