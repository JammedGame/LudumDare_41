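; Hand Blueprint that plays idle and spell-casting animations on its skeletal mesh.
; Separate events set the idle animation or one of three spell animations directly on the mesh.
; The spell events share a CanCast flag that blocks new casts until a one-second delay ends, while idle ignores it.
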(event Custom|Play%20idle
  ;[1 1 1] Idle
  (Components|Animation|SetAnimation (Variables|Default|GetSkeletalMesh) "/Game/Art/Meshes/Hand/A_Hand_Idle_Anim.A_Hand_Idle_Anim"))

(event Custom|Play%20Spell%202
  ;[1 1 1] Spell 2
  (if (Variables|Default|GetcanCast)
    (Variables|Default|SetcanCast false)
    (Components|Animation|SetAnimation (Variables|Default|GetSkeletalMesh) "/Game/Art/Meshes/Hand/Spell_02.Spell_02")
    (Utilities|FlowControl|Delay 1.0)
    (Variables|Default|SetcanCast true)))

(event Custom|Play%20Spell%203
  ;[1 1 1] Spell 3
  (if (Variables|Default|GetcanCast)
    (Variables|Default|SetcanCast false)
    (Components|Animation|SetAnimation (Variables|Default|GetSkeletalMesh) "/Game/Art/Meshes/Hand/Spell_03.Spell_03")
    (Utilities|FlowControl|Delay 1.0)
    (Variables|Default|SetcanCast true)))

(event Custom|Play%20Spell%201
  ;[1 1 1] Spell 1
  (if (Variables|Default|GetcanCast)
    (Variables|Default|SetcanCast false)
    (Components|Animation|SetAnimation (Variables|Default|GetSkeletalMesh) "/Game/Art/Meshes/Hand/Spell_01.Spell_01")
    (Utilities|FlowControl|Delay 1.0)
    (Variables|Default|SetcanCast true)))

(fn ConstructionScript)